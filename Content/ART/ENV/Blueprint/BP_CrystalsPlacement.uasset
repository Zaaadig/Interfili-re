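; BP_CrystalsPlacement procedurally scatters crystal meshes over a small flat square in its construction script.
; It builds one instanced static mesh component per SMList entry and records each mesh's bounding-box size, though placement ignores it.
; A seeded stream picks mesh, position and near-quarter-turn yaw per instance; the first two meshes get random reduced scale, others a fixed enlarged one.
; Leftover middle/top stacking logic is never executed.
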(fn `UserConstructionScript`
  (locals (ISM_List :type "Array of InstancedStaticMeshComponent Object Reference") (BB_List_X :type "Array of Float (double-precision)") (BB_List_Y :type "Array of Float (double-precision)") (BB_List_Z :type "Array of Float (double-precision)") (Actual_Index_Listes :type Integer) (Actual_ISM :type "InstancedStaticMeshComponent Object Reference") (L_Stone_SizeX :type "Float (double-precision)") (L_Stone_SizeY :type "Float (double-precision)") (L_Stone_SizeZ :type "Float (double-precision)") (FirstIndex :type Integer) (L_Index :type Integer) (Actual_Index_Instantiation :type Integer) (L_Stone_location :type "Vector Structure") (L_Stone_Rotation :type "Rotator Structure") (L_Stone_Size :type "Vector Structure") (FirstElt :type Integer) (ActualCrystal :type "InstancedStaticMeshComponent Object Reference"))
  (bind _stream (`self.Stream`))
  (bind _returnvalue (`KismetMathLibrary.RandomFloatInRangeFromStream` (`self.Stream`) 0.3 0.6))
  (bind (_returnvalue_min _returnvalue_max) (break `Box` (`StaticMesh.GetBoundingBox` (`|GetArrayItem` (`self.SM_List`) (`local.Actual_Index_Listes`)))))
  (`KismetArrayLibrary.Array_Clear` (`local.ISM_List`))
  (`KismetArrayLibrary.Array_Clear` (`local.BB_List_X`))
  (`KismetArrayLibrary.Array_Clear` (`local.BB_List_Y`))
  (`KismetArrayLibrary.Array_Clear` (`local.BB_List_Z`))
  (set `self.Stream` (`KismetMathLibrary.MakeRandomStream` (`self.Seed`)))
  (for _index (range (`KismetArrayLibrary.Array_Length` (`self.SM_List`)))
    (set `local.Actual_Index_Listes` _index)
    ;[1 1 1] Liste de SM liée a celle d'Instances
    (bind _returnvalue_2 (`AddComponent|NODE_AddInstancedStaticMeshComponent-0`))
    (bind _output_get (set `local.Actual_ISM` _returnvalue_2))
    (`StaticMeshComponent.SetStaticMesh` _output_get (`|GetArrayItem` (`self.SM_List`) (`local.Actual_Index_Listes`)))
    ;;[1 0 0] Ajout des Matériaux
    (`PrimitiveComponent.SetMaterial` (`local.Actual_ISM`) 0 null)
    (`KismetArrayLibrary.Array_Add` (`local.ISM_List`) (`local.Actual_ISM`))
    (bind _output_get_2 (set `local.L_Stone_SizeX` (.x (- _returnvalue_max _returnvalue_min))))
    (`KismetArrayLibrary.Array_Add` (`local.BB_List_X`) _output_get_2)
    (bind _output_get_3 (set `local.L_Stone_SizeY` (.y (- _returnvalue_max _returnvalue_min))))
    (`KismetArrayLibrary.Array_Add` (`local.BB_List_Y`) _output_get_3)
    (bind _output_get_4 (set `local.L_Stone_SizeZ` (.z (- _returnvalue_max _returnvalue_min))))
    (`KismetArrayLibrary.Array_Add` (`local.BB_List_Z`) _output_get_4))
  (for _index_2 (range (`local.FirstIndex`) (`self.Nbr_Pierres`))
    (set `local.L_Index` _index_2)
    (set `local.ActualCrystal` (`|GetArrayItem` (`local.ISM_List`) (`KismetMathLibrary.RandomIntegerInRangeFromStream` (`self.Stream`) 0 (`KismetArrayLibrary.Array_Length` (`local.ISM_List`)))))
    ;[1 0.7745 0] Position des SM
    (set `local.L_Stone_location` (`KismetMathLibrary.MakeVector` (`KismetMathLibrary.RandomFloatInRangeFromStream` _stream 0.0 200.0) (`KismetMathLibrary.RandomFloatInRangeFromStream` _stream 0.0 200.0)))
    ;[1 0 0.9783] Rotation des pierres
    (set `local.L_Stone_Rotation` (`KismetMathLibrary.ComposeRotators` (`KismetMathLibrary.MakeRotator` 0.0 0.0 (`KismetMathLibrary.Conv_IntToDouble` (* (`KismetMathLibrary.RandomIntegerInRangeFromStream` (`self.Stream`) -3 3) 90))) (`KismetMathLibrary.MakeRotator` 0.0 0.0 (`KismetMathLibrary.RandomFloatInRangeFromStream` (`self.Stream`) -5.0 5.0))))
    (if (or (== (`local.ActualCrystal`) (`|GetArrayItem` (`local.ISM_List`))) (== (`local.ActualCrystal`) (`|GetArrayItem` (`local.ISM_List`) 1)))
      ;[0 1 0.4702] Size des pierres
      (set `local.L_Stone_Size` (`KismetMathLibrary.MakeVector` _returnvalue _returnvalue _returnvalue))
      (else
        (set `local.L_Stone_Size` (5.0 5.0 5.0))))
    ;[0 0.01 1] Instancier la base
    (`InstancedStaticMeshComponent.AddInstance` (`local.ActualCrystal`) (`KismetMathLibrary.MakeTransform` (`local.L_Stone_location`) (`local.L_Stone_Rotation`) (`local.L_Stone_Size`)) false)))