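; Light switch trigger that changes the mood of every BP_RoofLight in the level while an actor overlaps it.
; On overlap begin it plays a switch sound, raises a scalar in the MPC_Light parameter collection, blacks out the roof lights, then after a short delay relights them dimmer at a very low, warm color temperature.
; On overlap end it resets the scalar and restores brighter, neutral-white lighting.
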(event `self.ReceiveActorBeginOverlap`
  (params (OtherActor :type "Actor Object Reference"))
  (`GameplayStatics.PlaySound2D` "/Game/ART/ENV/Sounds/Big_switch_sound_effect.Big_switch_sound_effect" 0.6 1.0 0.1 null null)
  (`KismetMaterialLibrary.SetScalarParameterValue` "/Game/ART/ENV/MeshesClean/UsineProps/MPC_Light.MPC_Light" "Prout" 1.0)
  (bind _outactors (`GameplayStatics.GetAllActorsOfClass` "/Game/ART/ENV/Blueprint/BP_RoofLight.BP_RoofLight_C"))
  (for _array_element _outactors
    (`LightComponent.SetIntensity` (`/Game/ART/ENV/Blueprint/BP_RoofLight.RectLight` _array_element) 0.0))
  (`KismetSystemLibrary.Delay` 0.2)
  (for _array_element_2 _outactors
    (bind _rectlight (`/Game/ART/ENV/Blueprint/BP_RoofLight.RectLight` _array_element_2))
    (`LightComponent.SetTemperature` _rectlight 10.0)
    (`LightComponent.SetIntensity` _rectlight 100.0)))

(event `self.ReceiveActorEndOverlap`
  (params (OtherActor :type "Actor Object Reference"))
  (`KismetMaterialLibrary.SetScalarParameterValue` "/Game/ART/ENV/MeshesClean/UsineProps/MPC_Light.MPC_Light" "Prout")
  (bind _outactors (`GameplayStatics.GetAllActorsOfClass` "/Game/ART/ENV/Blueprint/BP_RoofLight.BP_RoofLight_C"))
  (for _array_element _outactors
    (bind _rectlight (`/Game/ART/ENV/Blueprint/BP_RoofLight.RectLight` _array_element))
    (`LightComponent.SetTemperature` _rectlight 6500.0)
    (`LightComponent.SetIntensity` _rectlight 210.0)))

(fn `UserConstructionScript`)