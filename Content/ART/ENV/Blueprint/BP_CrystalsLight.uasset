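; BP_CrystalsLight is a crystal light actor whose point light brightens as an overlapping actor approaches.
; The sphere collision radius sets the maximum range, and intensity scales linearly with proximity up to MaxLight, floored at MinLight.
; Instead of Tick, a looping timer drives the TickOptimised update, unpausing on overlap begin and pausing on overlap end.
; Any overlapping actor is stored as Player without filtering.
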(event `self.ReceiveBeginPlay`
  ;[0.193 0.4194 1] Création du timer
  (set `self.Distance max` (`SphereComponent.GetScaledSphereRadius` (`self.Sphere_Collision`)))
  (bind _returnvalue (`KismetSystemLibrary.K2_SetTimerDelegate` (`|CreateDelegate` :!event `TickOptimised`) 0.1 true true))
  (bind _output_get (set `self.TImer` _returnvalue))
  (`KismetSystemLibrary.K2_PauseTimerHandle` _output_get))

(event `self.ReceiveActorBeginOverlap`
  (params (OtherActor :type "Actor Object Reference"))
  (set `self.Player` OtherActor)
  (`KismetSystemLibrary.K2_UnPauseTimerHandle` (`self.TImer`)))

(event `self.ReceiveActorEndOverlap`
  (params (OtherActor :type "Actor Object Reference"))
  (`KismetSystemLibrary.K2_PauseTimerHandle` (`self.TImer`)))

(event `TickOptimised`
  (bind _returnvalue (* (/ (- (`self.Distance max`) (`self.GetDistanceTo` (`self.Player`) self)) (`self.Distance max`)) (`self.Max_Light`)))
  (if (< _returnvalue (`self.Min_Light`))
    (bind _output_get (set `self.New_Intensity` (`self.Min_Light`)))
    (else
      (set `self.New_Intensity` _returnvalue)))
  (`LightComponent.SetIntensity` (`self.PointLight`) _output_get))

(fn `UserConstructionScript`)