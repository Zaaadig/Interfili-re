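; Overlap-triggered actor that switches streamed sublevels from the cave (Grotte) to the factory (Usine) when an actor tagged Player enters it.
; It asynchronously loads the factory level and its lighting level, visible once loaded, and unloads both cave counterparts without blocking.
; The switch is one-way, with no return logic, and prints a debug message on trigger.
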(event `self.ReceiveActorBeginOverlap`
  (params (OtherActor :type "Actor Object Reference"))
  (if (`self.ActorHasTag` OtherActor "Player")
    (`KismetSystemLibrary.PrintString` "cHANGEMENT" true true (struct :`R` 1.0 :`G` 0.067182 :`B` 0.057234 :`A` 1.0))
    (`GameplayStatics.LoadStreamLevelBySoftObjectPtr` (`self.SubLevel_Usine`) true)
    (`GameplayStatics.LoadStreamLevelBySoftObjectPtr` (`self.SubLevel_Usine_Light`) true)
    (`GameplayStatics.UnloadStreamLevelBySoftObjectPtr` (`self.SubLevel_Grotte`))
    (`GameplayStatics.UnloadStreamLevelBySoftObjectPtr` (`self.SubLevel_Grotte_Light`))))

(fn `UserConstructionScript`)