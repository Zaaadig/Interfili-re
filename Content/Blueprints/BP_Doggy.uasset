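; BP_Doggy is an AI stalker dog that patrols waypoints, chases the player and can be lured by an orb's hit location.
; A Gate controls the patrol loop, which consumes a waypoint list from the end with random waits, then refills it.
; Entering its sphere starts a looping timer chase with steadily rising speed; exiting resumes patrol.
; A second trigger shows the death message and resets the orb, while random timers play idle sounds.
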(event `self.ReceiveBeginPlay`
  (bind _waypoint2 (`self.WayPoint2`))
  ;[1 1 1] create/clear waypoints for the partol, get the player chara for the player follow event
  (`self.IddleSound`)
  (`KismetArrayLibrary.Array_Clear` (`self.WayPoint2`))
  (set `self.UpdateSpeed` (`self.InitialSpeed`))
  (bind _returnvalue (`GameplayStatics.GetActorOfClass` "/Game/ThirdPerson/Blueprints/BP_ThirdPersonCharacter.BP_ThirdPersonCharacter_C"))
  (set `self.RefChara` _returnvalue)
  (for _array_element (`self.ListWaypoint`)
    (`KismetArrayLibrary.Array_Add` (`self.WayPoint2`) (`SceneComponent.K2_GetComponentLocation` (`Actor.RootComponent` _array_element)))
    (set `self.Current Waypoint` (`|GetArrayItem` _waypoint2 (`KismetArrayLibrary.Array_LastIndex` _waypoint2)))
    (`self.Patrol`)))

(event `Patrol`
  ;[1 1 1] Event that open the gate and make the ai start his patrol
  (`self.Start`)
  (`self.AI_Patrol`)
  (set `self.isAttackingPlayer?` false))

(event `AI_Patrol`
  (bind _waypoint2 (`self.WayPoint2`))
  (bind _waypoint2_2 (`self.WayPoint2`))
  ;[1 1 1] Patrol scipt -> make ai go to point a to point b, c etc.
  (`/Engine/EditorBlueprintResources/StandardMacros.Gate` true :!label _label
    (:`Exit`
      (set `CharacterMovementComponent.MaxWalkSpeed` (`self.InitialSpeed`) (`self.CharacterMovement`))
      (`|AIMoveTo` self (`self.Current Waypoint`) null
        (:`OnSuccess`
          (`KismetSystemLibrary.Delay` (`KismetMathLibrary.RandomFloatInRange` (`self.MinWaitTime`) (`self.MaxWaitTime`)))
          (set `self.Current Waypoint` (`|GetArrayItem` _waypoint2 (`KismetArrayLibrary.Array_LastIndex` _waypoint2)))
          (`KismetArrayLibrary.Array_Remove` _waypoint2_2 (`KismetArrayLibrary.Array_LastIndex` _waypoint2_2))
          (if (== (`KismetArrayLibrary.Array_Length` (`self.WayPoint2`)) 0)
            (`self.Reset Patrol`)
            (else
              (`self.AI_Patrol`))))
        (:`OnFail`
          (`self.Patrol`))))))

(event `Start`
  ;[1 1 1] Patrol scipt -> make ai go to point a to point b, c etc.
  (goto _label :!via `Open`))

(event `End`
  ;[1 1 1] Patrol scipt -> make ai go to point a to point b, c etc.
  (goto _label :!via `Close`))

(event `self.Sphere.OnComponentBeginOverlap`
  (params (OverlappedComponent :type "PrimitiveComponent Object Reference") (OtherActor :type "Actor Object Reference") (OtherComp :type "PrimitiveComponent Object Reference") (OtherBodyIndex :type Integer) (bFromSweep :type Boolean) (SweepResult :type "HitResult Structure (by ref)"))
  ;[1 1 1] When the player enter the AI range, the ai follow the player instead of patrol route
  (if (`self.ActorHasTag` OtherActor "Player")
    (`GameplayStatics.PlaySoundAtLocation` null (`self.K2_GetActorLocation` self) (struct) 1.0 1.0 0.0 null null null null)
    (set `self.isAttackingPlayer?` true)
    (`self.End`)
    (`self.TrackPlayer`)))

(event `self.Sphere.OnComponentEndOverlap`
  (params (OverlappedComponent :type "PrimitiveComponent Object Reference") (OtherActor :type "Actor Object Reference") (OtherComp :type "PrimitiveComponent Object Reference") (OtherBodyIndex :type Integer))
  ;[1 1 1] When player exit the AI range, AI return to normal patrol route
  (if (`self.ActorHasTag` OtherActor "Player")
    (`GameplayStatics.PlaySoundAtLocation` null (`self.K2_GetActorLocation` self) (struct) 1.0 1.0 0.0 null null null null)
    (`KismetSystemLibrary.K2_ClearAndInvalidateTimerHandle` (stale `TrackPlayer` _returnvalue))
    (set `self.UpdateSpeed` (`self.InitialSpeed`))
    (`self.Patrol`)))

(event `TrackPlayer`
  ;[1 1 1] When player is in range - > stalker's speed increase
  (bind _returnvalue (`KismetSystemLibrary.K2_SetTimerDelegate` (delegate `Le code`) 0.1 true)))

(event `Le code`
  (bind _refchara (`self.RefChara`))
  ;[1 1 1] When player is in range - > stalker's speed increase
  (`KismetSystemLibrary.PrintString` (`KismetStringLibrary.Conv_DoubleToString` (`self.UpdateSpeed`)))
  (set `CharacterMovementComponent.MaxWalkSpeed` (`self.UpdateSpeed`) (`self.CharacterMovement`))
  (set `self.UpdateSpeed` (+ (`self.UpdateSpeed`) (`self.AddedNewSpeed`)))
  (`|AIMoveTo` self (`self.K2_GetActorLocation` _refchara) _refchara))

(event `Reset Patrol`
  ;[1 1 1] Boucle Patrol
  (`KismetArrayLibrary.Array_Clear` (`self.WayPoint2`))
  (for _array_element (`self.ListWaypoint`)
    (`KismetArrayLibrary.Array_Add` (`self.WayPoint2`) (`SceneComponent.K2_GetComponentLocation` (`Actor.RootComponent` _array_element)))
    (`self.Patrol`)))

(event `self.PlayerDeath.OnComponentBeginOverlap`
  (params (OverlappedComponent :type "PrimitiveComponent Object Reference") (OtherActor :type "Actor Object Reference") (OtherComp :type "PrimitiveComponent Object Reference") (OtherBodyIndex :type Integer) (bFromSweep :type Boolean) (SweepResult :type "HitResult Structure (by ref)"))
  ;[1 1 1] When player enter range player die (print)
  (if (`self.ActorHasTag` OtherActor "Player")
    (`GameplayStatics.PlaySoundAtLocation` null (`self.K2_GetActorLocation` (`GameplayStatics.GetPlayerController` 0)) (struct) 1.0 1.0 0.0 null null null null)
    ;[1 1 1] Die
    (bind _returnvalue (`GameplayStatics.GetActorOfClass` "/Game/ThirdPerson/Blueprints/BP_ThirdPersonCharacter.BP_ThirdPersonCharacter_C"))
    (message `/Game/Blueprints/BPI/BPI_Character.YouDie` _returnvalue)
    (bind _returnvalue_2 (`GameplayStatics.GetActorOfClass` "/Game/Blueprints/BP_Orb.BP_Orb_C"))
    (message `/Game/Blueprints/BPI/BPI_ResetOrbe.ResetOrbe` _returnvalue_2)))

(event `IddleSound`
  ;[1 1 1] Son Idle Dog
  (bind _returnvalue (`KismetSystemLibrary.K2_SetTimerDelegate` (delegate `CodeSound`) (`KismetMathLibrary.RandomFloatInRange` 10.0 20.0))))

(event `CodeSound`
  ;[1 1 1] Son Idle Dog
  (`GameplayStatics.PlaySoundAtLocation` "/Game/Audio/SFX/Player/SoundCue/SC_Doggy.SC_Doggy" (`self.K2_GetActorLocation` self) (struct) 1.0 1.0 0.0 null null null null)
  (if (`self.isAttackingPlayer?`)
    (`KismetSystemLibrary.K2_ClearAndInvalidateTimerHandle` (stale `IddleSound` _returnvalue))
    (else
      (`self.IddleSound`))))

(event `OrbEntendu`
  (bind _returnvalue (`KismetSystemLibrary.K2_SetTimerDelegate` (delegate `OrbEntendu`) 0.1))
  (`KismetSystemLibrary.K2_ClearAndInvalidateTimerHandle` _returnvalue)
  (`|AIMoveTo` self (`NavigationSystemV1.K2_ProjectPointToNavigation` (stale `/Game/Blueprints/BPI/BPI_Doggy.AttirerDoggy` LocHitOrb) null null (1500.0 1500.0 1500.0)) null
    (:`OnSuccess`
      (`KismetSystemLibrary.Delay` 5.0)
      (`self.Reset Patrol`)
      (`KismetSystemLibrary.PrintString` "Hello" true true (struct :`R` 0.065077 :`G` 1.0 :`A` 1.0)))
    (:`OnFail`
      (`self.Reset Patrol`)
      (`KismetSystemLibrary.PrintString` "Hello" true true (struct :`R` 1.0 :`G` 0.032249 :`A` 1.0)))))

(event `/Game/Blueprints/BPI/BPI_Doggy.AttirerDoggy`
  (params (LocHitOrb :type "Vector Structure"))
  (`self.OrbEntendu`))

(fn `UserConstructionScript`
  (`KismetArrayLibrary.Array_Clear` (`self.WayPoint2`)))