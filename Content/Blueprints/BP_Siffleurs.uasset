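; BP_Siffleurs is a "whistler" world object that, when destroyed, draws nearby enemies to its location.
; Each tick it projects its position to the screen and sets IsLookingAtWhistler according to whether that lies within the viewport, after casting to BP_Orb.
; DestroySiffleur plays a one-shot sound, messages BP_EnnemiAIBase actors within range, and hides the mesh and disables collision after a delay.
; RespawnSiffleurs restores the mesh and refreshes the enemy list.
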(event `self.ReceiveBeginPlay`)

(event `self.ReceiveTick`
  (params (DeltaSeconds :type "Float (single-precision)"))
  (bind (_returnvalue_x _returnvalue_y) (`KismetMathLibrary.BreakVector2D` (`WidgetLayoutLibrary.GetViewportSize`)))
  (bind _screenlocation (`PlayerController.ProjectWorldLocationToScreen` (`GameplayStatics.GetPlayerController` 0) (`self.K2_GetActorLocation`) false))
  ;[1 1 1] Detection position siffleurs à lécran
  (if (and (> (`KismetMathLibrary.BreakVector2D` _screenlocation) 0.0) (> (`.Y` (`KismetMathLibrary.BreakVector2D` _screenlocation)) 0.0) (< (`KismetMathLibrary.BreakVector2D` _screenlocation) _returnvalue_x) (< (`.Y` (`KismetMathLibrary.BreakVector2D` _screenlocation)) _returnvalue_y))
    (castclass `/Game/Blueprints/BP_Orb` "/Game/Blueprints/BP_Orb.BP_Orb_C")
    (set `self.IsLookingAtWhistler` true)
    (else
      (castclass `/Game/Blueprints/BP_Orb` "/Game/Blueprints/BP_Orb.BP_Orb_C")
      (set `self.IsLookingAtWhistler` false))))

(event `/Game/Blueprints/BPI/BPI_Siffleurs.DestroySiffleur`
  ;[1 1 1] Kill Siffleurs
  (set `self.SiffleursIsAttack` true)
  (`|ExecutionSequence`
    (:`then_0`
      (`KismetSystemLibrary.Delay` 2.0)
      (`ActorComponent.Deactivate` (`self.DefaultSceneRoot`))
      (`SceneComponent.SetVisibility` (`self.Mesh`) false false)
      (`PrimitiveComponent.SetCollisionEnabled` (`self.Mesh`) "NoCollision")
      (set `self.SiffleursIsAttack` false))
    (:`then_1`
      (`/Engine/EditorBlueprintResources/StandardMacros.DoOnce` false
        (:`Completed`
          (`GameplayStatics.PlaySoundAtLocation` "/Game/Audio/SFX/Player/SoundCue/SC_Siffleurs.SC_Siffleurs" (`SceneComponent.K2_GetComponentLocation` (`self.DefaultSceneRoot`)) (struct) 1.0 1.0 0.0 null null null null))))
    (:`then_2`
      (bind _outactors (`GameplayStatics.GetAllActorsOfClass` "/Game/Blueprints/BP_EnnemiAIBase.BP_EnnemiAIBase_C"))
      (bind _output_get (set `self.AllEnnemi` _outactors))
      (for _array_element _output_get
        (if (< (`self.GetDistanceTo` _array_element self) 2000.0)
          (`KismetArrayLibrary.Array_Add` (`self.ListInRange`) _array_element)
          (message `/Game/Blueprints/BPI/BPI_Siffleurs.AttirerSiffleurs` (`self.ListInRange`) (`self.K2_GetActorLocation`)))))))

(event `/Game/Blueprints/BPI/BPI_Siffleurs.RespawnSiffleurs`
  (`KismetArrayLibrary.Array_Clear` (`self.AllEnnemi`))
  (`ActorComponent.Activate` (`self.DefaultSceneRoot`) false)
  (`SceneComponent.SetVisibility` (`self.Mesh`) true false)
  (`PrimitiveComponent.SetCollisionEnabled` (`self.Mesh`) "QueryAndPhysics")
  (bind _outactors (`GameplayStatics.GetAllActorsOfClass` "/Game/Blueprints/BP_EnnemiAIBase.BP_EnnemiAIBase_C"))
  (set `self.AllEnnemi` _outactors))

(fn `UserConstructionScript`)