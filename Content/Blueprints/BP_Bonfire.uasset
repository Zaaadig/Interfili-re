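; BP_Bonfire is a checkpoint bonfire that restores life to the player character.
; While the player flag from collider overlaps and IsInteract are both true, Tick calls ActivateBonfire.
; Activation applies a red dynamic material, sets PlayerLife on the cached BP_ThirdPersonCharacter, flags HealOrb after a BP_Orb cast, and sends the bonfire's location via BonfireActivatedMessage.
; Overlap events do not filter by actor, and activation repeats each qualifying tick.
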(event `self.ReceiveBeginPlay`
  ;[1 1 1] Initailisation
  (bind _returnvalue (`GameplayStatics.GetActorOfClass` "/Game/ThirdPerson/Blueprints/BP_ThirdPersonCharacter.BP_ThirdPersonCharacter_C"))
  (set `self.CharaRef` _returnvalue))

(event `self.ReceiveTick`
  (params (DeltaSeconds :type "Float (single-precision)"))
  ;[1 1 1] Checking
  (if (`self.isPlayerHere?`)
    (if (`self.isInteract?`)
      (`self.Activate Bonfire`))))

(event `self.Collider.OnComponentBeginOverlap`
  (params (OverlappedComponent :type "PrimitiveComponent Object Reference") (OtherActor :type "Actor Object Reference") (OtherComp :type "PrimitiveComponent Object Reference") (OtherBodyIndex :type Integer) (bFromSweep :type Boolean) (SweepResult :type "HitResult Structure (by ref)"))
  ;[1 1 1] Set Bool
  (set `self.isPlayerHere?` true))

(event `self.Collider.OnComponentEndOverlap`
  (params (OverlappedComponent :type "PrimitiveComponent Object Reference") (OtherActor :type "Actor Object Reference") (OtherComp :type "PrimitiveComponent Object Reference") (OtherBodyIndex :type Integer))
  ;[1 1 1] Set Bool
  (set `self.isPlayerHere?` false))

(event `Activate Bonfire`
  ;[0.9429 0.7035 1 0.4 14] Change Color When Activated
  (bind _returnvalue (`PrimitiveComponent.CreateDynamicMaterialInstance` (`self.StaticMesh`) 0 "/Game/StarterContent/Materials/M_Basic_Wall.M_Basic_Wall" "None"))
  (`MaterialInstanceDynamic.SetVectorParameterValue` _returnvalue "Base Color" (struct :`R` 0.536458 :`G` 0.016764 :`B` 0.016764 :`A` 1.0))
  ;[0.4133 1 0.4646 0.753] Life Recovery
  (bind _output_get (set `self.OrbLife` 200.0))
  (castclass `/Game/ThirdPerson/Blueprints/BP_ThirdPersonCharacter` "/Game/ThirdPerson/Blueprints/BP_ThirdPersonCharacter.BP_ThirdPersonCharacter_C")
  (set `/Game/ThirdPerson/Blueprints/BP_ThirdPersonCharacter.PlayerLife` _output_get (`self.CharaRef`))
  (castclass `/Game/Blueprints/BP_Orb` "/Game/Blueprints/BP_Orb.BP_Orb_C")
  (set `self.HealOrb?` true)
  ;[1 0.5541 0.2357 0.657] CheckpointLoc
  (bind _output_get_2 (set `self.Checkpoint` (`SceneComponent.K2_GetComponentLocation` (`self.DefaultSceneRoot`))))
  (`KismetSystemLibrary.PrintString` (`KismetStringLibrary.Conv_DoubleToString` _output_get))
  (`KismetSystemLibrary.PrintString` (`KismetStringLibrary.Conv_VectorToString` _output_get_2))
  (message `/Game/Blueprints/BPI_Character.BonfireActivated` (`self.CharaRef`) (`self.Checkpoint`)))

(fn `UserConstructionScript`)