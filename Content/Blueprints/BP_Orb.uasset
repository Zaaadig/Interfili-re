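; BP_Orb is a light orb that fades over its lifetime, then refills after a short delay or whenever a bonfire heals it.
; A looping timer shrinks its light, MPC_Fog size and detection sphere together, while Tick publishes its position to MPC_Orb.
; Sphere overlaps with Siffleurs trigger line-of-sight checks that destroy watching whistlers the player can see.
; Hard impacts play a sound and lure nearby Doggies to the orb.
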(event `self.ReceiveBeginPlay`
  (bind _light_vie (`self.Light_Vie`))
  (bind (_returnvalue_location _returnvalue_rotation _returnvalue_scale) (`KismetMathLibrary.BreakTransform` (`SceneComponent.GetRelativeTransform` (`self.Sphere Collision`))))
  ;[1 1 1] Begin Play
  (bind _outactors (`GameplayStatics.GetAllActorsOfClass` "/Game/Blueprints/BP_Bonefire.BP_Bonefire_C"))
  (set `self.AllBonfire` _outactors)
  (bind _outactors_2 (`GameplayStatics.GetAllActorsOfClass` "/Game/Blueprints/BP_Siffleurs.BP_Siffleurs_C"))
  (bind _returnvalue (`GameplayStatics.GetActorOfClass` "/Game/ThirdPerson/Blueprints/BP_ThirdPersonCharacter.BP_ThirdPersonCharacter_C"))
  (set `self.RefChara` _returnvalue)
  (set `self.RefSiffleur` _outactors_2)
  (bind _output_get (set `self.CurrentIntensity` (`self.BaseIntensity`)))
  (`LightComponent.SetIntensity` _light_vie _output_get)
  (bind _output_get_2 (set `self.CurrentRadius` (`self.BaseRadius`)))
  (`LocalLightComponent.SetAttenuationRadius` _light_vie _output_get_2)
  (`self.StartTimerLife`)
  (bind _output_get_3 (set `self.TranformCollision` _returnvalue_scale))
  (set `self.UpdateTransformCollision` _output_get_3)
  (bind _outactors_3 (`GameplayStatics.GetAllActorsOfClass` "/Game/Blueprints/BP_Doggy.BP_Doggy_C"))
  (set `self.AllDoggyRef` _outactors_3)
  (bind _output_get_4 (set `self.BaseFog` 750.0))
  (set `self.CurrentFog` _output_get_4))

(event `StartTimerLife`
  ;[1 1 1] Gestion Intensité Couleur / Taille
  (bind _returnvalue (`KismetSystemLibrary.K2_SetTimerDelegate` (delegate `LifeVisual`) 0.1 true)))

(event `LifeVisual`
  (bind _sphere_collision (`self.Sphere Collision`))
  (bind (_returnvalue_location _returnvalue_rotation) (`KismetMathLibrary.BreakTransform` (`SceneComponent.GetRelativeTransform` _sphere_collision)))
  (bind _returnvalue (- (`self.UpdateTransformCollision`) (/ (`self.TranformCollision`) (`self.LifeTime`))))
  ;[1 1 1] Gestion Intensité Couleur / Taille
  (bind _output_get (set `self.CurrentIntensity` (- (`self.CurrentIntensity`) (/ (`self.BaseIntensity`) (`self.LifeTime`)))))
  (`LightComponent.SetIntensity` (`self.Light_Vie`) _output_get)
  (bind _output_get_2 (set `self.CurrentRadius` (- (`self.CurrentRadius`) (/ (`self.BaseRadius`) (`self.LifeTime`)))))
  (`LocalLightComponent.SetAttenuationRadius` (`self.Light_Vie`) _output_get_2)
  (bind _output_get_3 (set `self.CurrentFog` (- (`self.CurrentFog`) (/ (`self.BaseFog`) (`self.LifeTime`)))))
  (`KismetMaterialLibrary.SetScalarParameterValue` "/Game/ART/ENV/Materials/MM/MPC_Fog.MPC_Fog" "Fog_Size" _output_get_3)
  (set `self.UpdateTransformCollision` _returnvalue)
  (`SceneComponent.K2_SetRelativeTransform` _sphere_collision (`KismetMathLibrary.MakeTransform` _returnvalue_location _returnvalue_rotation _returnvalue) false false)
  (if (<= (`self.CurrentRadius`) 0.0)
    ;[1 1 1] Begin Play
    (`KismetSystemLibrary.K2_ClearAndInvalidateTimerHandle` (stale `StartTimerLife` _returnvalue))
    (`self.RestartHere`)))

(event `RestartHere`
  ;[1 1 1] Gestion Intensité Couleur / Taille
  (`KismetSystemLibrary.Delay` 2.0 :!label _label)
  (set `self.CurrentIntensity` (`self.BaseIntensity`))
  (set `self.CurrentRadius` (`self.BaseRadius`))
  (set `self.CurrentFog` (`self.BaseFog`))
  (set `self.UpdateTransformCollision` (`self.TranformCollision`))
  (`self.StartTimerLife`))

(event `/Game/Blueprints/BPI/BPI_Restart.Restart`
  ;[1 1 1] Gestion Intensité Couleur / Taille
  (goto _label))

(event `self.Sphere Collision.OnComponentBeginOverlap`
  (params (OverlappedComponent :type "PrimitiveComponent Object Reference") (OtherActor :type "Actor Object Reference") (OtherComp :type "PrimitiveComponent Object Reference") (OtherBodyIndex :type Integer) (bFromSweep :type Boolean) (SweepResult :type "HitResult Structure (by ref)"))
  ;[1 1 1] Détéction siffleurs
  (if (`self.ActorHasTag` OtherActor "Siffleur")
    (for _array_element (`self.RefSiffleur`)
      (if (`/Game/Blueprints/BP_Siffleurs.IsLookingAtWhistler` _array_element)
        (if (`Controller.LineOfSightTo` (`GameplayStatics.GetPlayerController` 0) _array_element (0.0 0.0 0.0) false)
          (set `self.PayerCanSeeWhistler` true)
          (message `/Game/Blueprints/BPI/BPI_Siffleurs.DestroySiffleur` _array_element)
          (else
            (set `self.PayerCanSeeWhistler` false)))))))

(event `self.ReceiveTick`
  (params (DeltaSeconds :type "Float (single-precision)"))
  ;[1 1 1] Rechargement vie visuel
  (`KismetMaterialLibrary.SetVectorParameterValue` "/Game/LevelPrototyping/MPC_Orb.MPC_Orb" "OrbPosition" (`KismetMathLibrary.Conv_VectorToLinearColor` (`self.K2_GetActorLocation`)))
  (for _array_element (`self.AllBonfire`)
    (if (`/Game/Blueprints/BP_Bonefire.HealOrb?` _array_element)
      (set `self.CurrentIntensity` (`self.BaseIntensity`) :!label _label_2)
      (set `self.CurrentRadius` (`self.BaseRadius`))
      (set `self.UpdateTransformCollision` (`self.TranformCollision`))
      (set `/Game/Blueprints/BP_Bonefire.HealOrb?` false _array_element))))

(event `/Game/Blueprints/BPI/BPI_ResetOrbe.ResetOrbe`
  ;[1 1 1] Rechargement vie visuel
  (goto _label_2))

(event `self.Sphere.OnComponentHit`
  (params (HitComponent :type "PrimitiveComponent Object Reference") (OtherActor :type "Actor Object Reference") (OtherComp :type "PrimitiveComponent Object Reference") (NormalImpulse :type "Vector Structure") (Hit :type "HitResult Structure (by ref)"))
  (bind _doggyinrange (`self.DoggyInRange`))
  (bind _returnvalue (`self.K2_GetActorLocation` self))
  (`PrimitiveComponent.SetSimulatePhysics` (`self.Sphere`) false)
  (if (not (< (`KismetMathLibrary.VSize` NormalImpulse) 400.0))
    (`KismetSystemLibrary.Delay` 0.2)
    (`GameplayStatics.PlaySoundAtLocation` "/Game/Audio/SFX/Player/SoundCue/SC_OrbHit.SC_OrbHit" _returnvalue (struct) 1.0 1.0 0.0 null null null null)
    (for _array_element (`self.AllDoggyRef`)
      (if (< (`self.GetDistanceTo` _array_element self) 1500.0)
        (`KismetArrayLibrary.Array_Add` _doggyinrange _array_element)
        (message `/Game/Blueprints/BPI/BPI_Doggy.AttirerDoggy` _doggyinrange _returnvalue)
        (`KismetSystemLibrary.Delay` 0.4)
        (set `self.IsPlayingSound?` false)))))

(event `/Game/Blueprints/BPI/BPI_Switch.RecupDoggy`
  (params (DogList :type "Array of /Game/Blueprints/BP_Doggy Object Reference (by ref)"))
  (bind _outactors (`GameplayStatics.GetAllActorsOfClass` "/Game/Blueprints/BP_Doggy.BP_Doggy_C"))
  (set `self.AllDoggyRef` _outactors))

(fn `UserConstructionScript`
  (`KismetArrayLibrary.Array_Clear` (`self.Tags`))
  (`KismetArrayLibrary.Array_AddUnique` (`self.Tags`) "Orb"))