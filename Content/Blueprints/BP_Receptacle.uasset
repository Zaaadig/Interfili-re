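; BP_Receptacle is a trigger that reveals a set of demon platforms while an actor tagged "Orb" sits inside its box.
; Begin and end overlap store the tag check in BallHere and pass it to InvocarPlataformadelDemonio or Desinvocar.
; When the check is true, those events call SetVisible or SetInvisible on every element of PlateformArray.
; Begin overlap also prints a leftover debug string for any overlapping actor.
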(event `Invocar Plataforma del Demonio`
  (params (bIsOrb :type Boolean))
  (if bIsOrb
    (for _array_element (`self.Plateform_Array`)
      (`/Game/Blueprints/BP_Plateforme.Set Visible` _array_element))))

(event `Desinvocar`
  (params (bIsOrb :type Boolean))
  (if bIsOrb
    (for _array_element (`self.Plateform_Array`)
      (`/Game/Blueprints/BP_Plateforme.Set Invisible` _array_element))))

(event `self.Box.OnComponentBeginOverlap`
  (params (OverlappedComponent :type "PrimitiveComponent Object Reference") (OtherActor :type "Actor Object Reference") (OtherComp :type "PrimitiveComponent Object Reference") (OtherBodyIndex :type Integer) (bFromSweep :type Boolean) (SweepResult :type "HitResult Structure (by ref)"))
  (bind _output_get (set `self.ballHere?` (`self.ActorHasTag` OtherActor "Orb")))
  (`self.Invocar Plataforma del Demonio` _output_get)
  (`KismetSystemLibrary.PrintString` "dadaf"))

(event `self.Box.OnComponentEndOverlap`
  (params (OverlappedComponent :type "PrimitiveComponent Object Reference") (OtherActor :type "Actor Object Reference") (OtherComp :type "PrimitiveComponent Object Reference") (OtherBodyIndex :type Integer))
  (bind _output_get (set `self.ballHere?` (`self.ActorHasTag` OtherActor "Orb")))
  (`self.Desinvocar` _output_get))

(fn `UserConstructionScript`)