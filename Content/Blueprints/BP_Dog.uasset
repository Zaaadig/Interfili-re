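; BP_Dog is an enemy AI that patrols BP_WayPoint actors and chases the player who enters its detection sphere.
; A Gate controls the patrol loop, which walks the waypoint array from the end with random waits and refills it when empty.
; During a chase, a looping timer re-issues AIMoveTo with steadily rising speed until the player leaves the sphere.
; Overlapping the PlayerDeath volume triggers death and orb-reset messages.
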(event `self.ReceiveBeginPlay`
  (bind _waypoint (`self.WayPoint`))
  ;[1 1 1] create/clear waypoints for the partol, get the player chara for the player follow event
  (`KismetArrayLibrary.Array_Clear` (`self.WayPoint`))
  (set `self.UpdateSpeed` (`self.InitialSpeed`))
  (bind _returnvalue (`GameplayStatics.GetActorOfClass` "/Game/ThirdPerson/Blueprints/BP_ThirdPersonCharacter.BP_ThirdPersonCharacter_C"))
  (set `self.RefChara` _returnvalue)
  (bind _outactors (`GameplayStatics.GetAllActorsOfClass` "/Game/Blueprints/BP_WayPoint.BP_WayPoint_C"))
  (for _array_element _outactors
    (`KismetArrayLibrary.Array_Add` (`self.WayPoint`) (`SceneComponent.K2_GetComponentLocation` (`Actor.RootComponent` _array_element)))
    (set `self.Current Waypoint` (`|GetArrayItem` _waypoint (`KismetArrayLibrary.Array_LastIndex` _waypoint)))
    (`self.Patrol`)))

(event `Patrol`
  ;[1 1 1] Event that open the gate and make the ai start his patrol
  (`self.Start`)
  (`self.AI_Patrol`)
  (set `self.isAttackingPlayer?` false))

(event `AI_Patrol`
  (bind _waypoint (`self.WayPoint`))
  (bind _waypoint_2 (`self.WayPoint`))
  ;[1 1 1] Patrol scipt -> make ai go to point a to point b, c etc.
  (`/Engine/EditorBlueprintResources/StandardMacros.Gate` true :!label _label
    (:`Exit`
      (set `CharacterMovementComponent.MaxWalkSpeed` (`self.InitialSpeed`) (`self.CharacterMovement`))
      (`|AIMoveTo` self (`self.Current Waypoint`) null
        (:`OnSuccess`
          (`KismetSystemLibrary.Delay` (`KismetMathLibrary.RandomFloatInRange` (`self.MinWaitTime`) (`self.MaxWaitTime`)))
          (set `self.Current Waypoint` (`|GetArrayItem` _waypoint (`KismetArrayLibrary.Array_LastIndex` _waypoint)))
          (`KismetArrayLibrary.Array_Remove` _waypoint_2 (`KismetArrayLibrary.Array_LastIndex` _waypoint_2))
          (if (== (`KismetArrayLibrary.Array_Length` _waypoint_2) 0)
            (`self.Reset Patrol`)
            (else
              (`self.AI_Patrol`))))))))

(event `Start`
  ;[1 1 1] Patrol scipt -> make ai go to point a to point b, c etc.
  (goto _label :!via `Open`))

(event `End`
  ;[1 1 1] Patrol scipt -> make ai go to point a to point b, c etc.
  (goto _label :!via `Close`))

(event `self.Sphere.OnComponentBeginOverlap`
  (params (OverlappedComponent :type "PrimitiveComponent Object Reference") (OtherActor :type "Actor Object Reference") (OtherComp :type "PrimitiveComponent Object Reference") (OtherBodyIndex :type Integer) (bFromSweep :type Boolean) (SweepResult :type "HitResult Structure (by ref)"))
  ;[1 1 1] When the player enter the AI range, the ai follow the player instead of patrol route
  (if (`self.ActorHasTag` OtherActor "Player")
    (`GameplayStatics.PlaySoundAtLocation` null (`self.K2_GetActorLocation` self) (struct) 1.0 1.0 0.0 null null null null)
    (set `self.isAttackingPlayer?` true)
    (`self.End`)
    (`self.TrackPlayer`)))

(event `self.Sphere.OnComponentEndOverlap`
  (params (OverlappedComponent :type "PrimitiveComponent Object Reference") (OtherActor :type "Actor Object Reference") (OtherComp :type "PrimitiveComponent Object Reference") (OtherBodyIndex :type Integer))
  ;[1 1 1] When player exit the AI range, AI return to normal patrol route
  (if (`self.ActorHasTag` OtherActor "Player")
    (`GameplayStatics.PlaySoundAtLocation` null (`self.K2_GetActorLocation` self) (struct) 1.0 1.0 0.0 null null null null)
    (`KismetSystemLibrary.K2_ClearAndInvalidateTimerHandle` (stale `TrackPlayer` _returnvalue))
    (set `self.UpdateSpeed` (`self.InitialSpeed`))
    (`self.Patrol`)))

(event `TrackPlayer`
  ;[1 1 1] When player is in range - > stalker's speed increase
  (bind _returnvalue (`KismetSystemLibrary.K2_SetTimerDelegate` (delegate `Le code`) 0.1 true)))

(event `Le code`
  (bind _refchara (`self.RefChara`))
  ;[1 1 1] When player is in range - > stalker's speed increase
  (`KismetSystemLibrary.PrintString` (`KismetStringLibrary.Conv_DoubleToString` (`self.UpdateSpeed`)))
  (set `CharacterMovementComponent.MaxWalkSpeed` (`self.UpdateSpeed`) (`self.CharacterMovement`))
  (set `self.UpdateSpeed` (+ (`self.UpdateSpeed`) (`self.AddedNewSpeed`)))
  (`|AIMoveTo` self (`self.K2_GetActorLocation` _refchara) _refchara))

(event `Reset Patrol`
  ;[1 1 1] Boucle Patrol
  (`KismetArrayLibrary.Array_Clear` (`self.WayPoint`))
  (bind _outactors (`GameplayStatics.GetAllActorsOfClass` "/Game/Blueprints/BP_WayPoint.BP_WayPoint_C"))
  (for _array_element _outactors
    (`KismetArrayLibrary.Array_Add` (`self.WayPoint`) (`SceneComponent.K2_GetComponentLocation` (`Actor.RootComponent` _array_element)))
    (`self.Patrol`)))

(event `self.PlayerDeath.OnComponentBeginOverlap`
  (params (OverlappedComponent :type "PrimitiveComponent Object Reference") (OtherActor :type "Actor Object Reference") (OtherComp :type "PrimitiveComponent Object Reference") (OtherBodyIndex :type Integer) (bFromSweep :type Boolean) (SweepResult :type "HitResult Structure (by ref)"))
  ;[1 1 1] when player enter range player die (print)
  (if (`self.ActorHasTag` OtherActor "Player")
    (`GameplayStatics.PlaySoundAtLocation` null (`self.K2_GetActorLocation` (`GameplayStatics.GetPlayerController` 0)) (struct) 1.0 1.0 0.0 null null null null)
    ;[1 1 1] Die
    (bind _returnvalue (`GameplayStatics.GetActorOfClass` "/Game/ThirdPerson/Blueprints/BP_ThirdPersonCharacter.BP_ThirdPersonCharacter_C"))
    (message `/Game/Blueprints/BPI/BPI_Character.YouDie` _returnvalue)
    (bind _returnvalue_2 (`GameplayStatics.GetActorOfClass` "/Game/Blueprints/BP_Orb.BP_Orb_C"))
    (message `/Game/Blueprints/BPI/BPI_ResetOrbe.ResetOrbe` _returnvalue_2)))

(fn `UserConstructionScript`
  (`KismetArrayLibrary.Array_Clear` (`self.WayPoint`)))