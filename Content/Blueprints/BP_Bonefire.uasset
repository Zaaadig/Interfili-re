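; Bonfire checkpoint actor that heals the player and orb and records a respawn location.
; Collider overlap sets a player-present flag and fades the WB_Interact prompt, while Tick polls that flag and IsInteract to trigger activation.
; Activation brightens a dynamic emissive material, plays a sound, swaps the Niagara effect, restores player and orb life, resets the orb's fog, and sends the Sphere's location to the character as checkpoint.
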(event `self.ReceiveBeginPlay`
  ;[1 1 1] Initailisation
  (bind _returnvalue (`GameplayStatics.GetActorOfClass` "/Game/ThirdPerson/Blueprints/BP_ThirdPersonCharacter.BP_ThirdPersonCharacter_C"))
  (set `self.CharaRef` _returnvalue)
  (bind _returnvalue_2 (`|CreateWidget` "/Game/Blueprints/Widget/WB_Interact.WB_Interact_C"))
  (bind _output_get (set `self.Widget` _returnvalue_2))
  (`UserWidget.AddToViewport` _output_get 0)
  ;[1 1 1] Création et set de l'emissive
  (bind _returnvalue_3 (`PrimitiveComponent.CreateDynamicMaterialInstance` (`self.StaticMesh`) 0 "/Game/ART/ENV/Materials/MM/MM_BakedEmissivAsset.MM_BakedEmissivAsset" "None"))
  (bind _output_get_2 (set `self.DynamixMat_Ref` _returnvalue_3))
  (`MaterialInstanceDynamic.SetScalarParameterValue` _output_get_2 "Emissiv_Power" (`self.Base_Emissiv`))
  (bind _returnvalue_4 (`GameplayStatics.GetActorOfClass` "/Game/Blueprints/BP_Orb.BP_Orb_C"))
  (set `self.OrbRef` _returnvalue_4))

(event `self.ReceiveTick`
  (params (DeltaSeconds :type "Float (single-precision)"))
  ;[1 1 1] Checking
  (if (`self.isPlayerHere?`)
    (if (`self.isInteract?`)
      (`self.Activate Bonfire`))))

(event `self.Collider.OnComponentBeginOverlap`
  (params (OverlappedComponent :type "PrimitiveComponent Object Reference") (OtherActor :type "Actor Object Reference") (OtherComp :type "PrimitiveComponent Object Reference") (OtherBodyIndex :type Integer) (bFromSweep :type Boolean) (SweepResult :type "HitResult Structure (by ref)"))
  ;[1 1 1] Set Bool
  (set `self.isPlayerHere?` true)
  (if (`self.ActorHasTag` OtherActor "Player")
    (`Image.SetOpacity` (`/Game/Blueprints/Widget/WB_Interact.E` (`self.Widget`)) 1.0)))

(event `self.Collider.OnComponentEndOverlap`
  (params (OverlappedComponent :type "PrimitiveComponent Object Reference") (OtherActor :type "Actor Object Reference") (OtherComp :type "PrimitiveComponent Object Reference") (OtherBodyIndex :type Integer))
  ;[1 1 1] Set Bool
  (set `self.isPlayerHere?` false)
  (if (`self.ActorHasTag` OtherActor "Player")
    (`Image.SetOpacity` (`/Game/Blueprints/Widget/WB_Interact.E` (`self.Widget`)) 0.05)))

(event `Activate Bonfire`
  ;[0.9429 0.7035 1 0.4 14] Change Color When Activated
  (`MaterialInstanceDynamic.SetScalarParameterValue` (`self.DynamixMat_Ref`) "Emissiv_Power" 20.0)
  (`GameplayStatics.PlaySoundAtLocation` null (`self.K2_GetActorLocation` self) (struct) 1.0 1.0 0.0 null null null null)
  ;[0.4133 1 0.4646 0.753] Life Recovery
  (bind _output_get (set `self.OrbLife` 200.0))
  (castclass `/Game/ThirdPerson/Blueprints/BP_ThirdPersonCharacter` "/Game/ThirdPerson/Blueprints/BP_ThirdPersonCharacter.BP_ThirdPersonCharacter_C")
  (set `/Game/ThirdPerson/Blueprints/BP_ThirdPersonCharacter.PlayerLife` _output_get (`self.CharaRef`))
  (castclass `/Game/Blueprints/BP_Orb` "/Game/Blueprints/BP_Orb.BP_Orb_C")
  (set `self.HealOrb?` true)
  ;[1 0.5541 0.2357 0.657] CheckpointLoc
  (set `self.Checkpoint` (`SceneComponent.K2_GetComponentLocation` (`self.Sphere`)))
  (message `/Game/Blueprints/BPI/BPI_Character.BonfireActivated` (`self.CharaRef`) (`self.Checkpoint`))
  (`NiagaraComponent.SetAsset` (`self.Niagara`) "/Game/ART/NS/NS_Bonfire_activated.NS_Bonfire_activated" true)
  (castclass `/Game/Blueprints/BP_Orb` "/Game/Blueprints/BP_Orb.BP_Orb_C")
  (set `/Game/Blueprints/BP_Orb.CurrentFog` 750.0 (`self.OrbRef`)))

(fn `UserConstructionScript`)