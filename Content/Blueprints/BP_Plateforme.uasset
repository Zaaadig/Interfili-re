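; BP_Plateforme is a platform actor that can be toggled between a hidden, passable state and a visible, solid one.
; On BeginPlay its StaticMesh is hidden with collision disabled.
; The SetVisible event shows the mesh with query and physics collision, and SetInvisible returns it to the hidden state.
; The file contains no trigger logic, only these events.
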(event `self.ReceiveBeginPlay`
  (`SceneComponent.SetVisibility` (`self.StaticMesh`) false false)
  (`PrimitiveComponent.SetCollisionEnabled` (`self.StaticMesh`) "NoCollision"))

(event `Set Visible`
  (`SceneComponent.SetVisibility` (`self.StaticMesh`) true false)
  (`PrimitiveComponent.SetCollisionEnabled` (`self.StaticMesh`) "QueryAndPhysics"))

(event `Set Invisible`
  (`SceneComponent.SetVisibility` (`self.StaticMesh`) false false)
  (`PrimitiveComponent.SetCollisionEnabled` (`self.StaticMesh`) "NoCollision"))

(fn `UserConstructionScript`)