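; BP_CaveAmbient is a cave ambience actor that plays 2D ambient and wind sounds at random intervals.
; BeginPlay starts two randomized timers, a long one for ambience and a short one for wind.
; Box overlaps with Player-tagged actors only set PlayerIsIn.
; Each timer plays its sound, then re-arms only while that flag is true, so a stopped loop stays stopped when the player re-enters.
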(event `self.ReceiveBeginPlay`
  ;[1 1 1] Init
  (`self.StartLoop`)
  (`self.StartLoopWind`))

(event `self.Box.OnComponentBeginOverlap`
  (params (OverlappedComponent :type "PrimitiveComponent Object Reference") (OtherActor :type "Actor Object Reference") (OtherComp :type "PrimitiveComponent Object Reference") (OtherBodyIndex :type Integer) (bFromSweep :type Boolean) (SweepResult :type "HitResult Structure (by ref)"))
  ;[1 1 1] Gestion d'état
  (if (`self.ActorHasTag` OtherActor "Player")
    (set `self.PlayerIsIn?` true)))

(event `self.Box.OnComponentEndOverlap`
  (params (OverlappedComponent :type "PrimitiveComponent Object Reference") (OtherActor :type "Actor Object Reference") (OtherComp :type "PrimitiveComponent Object Reference") (OtherBodyIndex :type Integer))
  ;[1 1 1] Gestion d'état
  (if (`self.ActorHasTag` OtherActor "Player")
    (set `self.PlayerIsIn?` false)))

(event `StartLoop`
  ;[1 1 1] Loop pendant qu'on est dans la box
  (bind _returnvalue (`KismetSystemLibrary.K2_SetTimerDelegate` (delegate `Loop`) (`KismetMathLibrary.RandomFloatInRange` 90.0 150.0))))

(event `Loop`
  ;[1 1 1] Loop pendant qu'on est dans la box
  (`GameplayStatics.PlaySound2D` "/Game/Audio/SFX/Ambiance/SC_Ambient.SC_Ambient" 1.0 1.0 0.0 null null)
  (if (`self.PlayerIsIn?`)
    (`self.StartLoop`)
    (else
      (`KismetSystemLibrary.K2_ClearAndInvalidateTimerHandle` (stale `StartLoop` _returnvalue)))))

(event `StartLoopWind`
  ;[1 1 1] Wind Loop
  (bind _returnvalue (`KismetSystemLibrary.K2_SetTimerDelegate` (delegate `LoopWind`) (`KismetMathLibrary.RandomFloatInRange` 2.5 5.0))))

(event `LoopWind`
  ;[1 1 1] Wind Loop
  (`GameplayStatics.PlaySound2D` "/Game/Audio/SFX/Ambiance/SC_Wind2.SC_Wind2" 1.0 1.0 0.0 null null)
  (if (`self.PlayerIsIn?`)
    (`self.StartLoopWind`)
    (else
      (`KismetSystemLibrary.K2_ClearAndInvalidateTimerHandle` (stale `StartLoopWind` _returnvalue)))))

(fn `UserConstructionScript`)