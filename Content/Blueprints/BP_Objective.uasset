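; BP_Objective is an objective actor that signals the final door when the player is near.
; BeginPlay caches the third-person character and BP_FinalDoor.
; Collision overlaps with Player-tagged actors toggle PlayerIsNear, with a debug print on entry.
; Tick calls the door's OpenDoorMessage every frame while PlayerIsNear and PlayerCanInteract are true, though PlayerCanInteract is not set in this graph.
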(event `self.ReceiveBeginPlay`
  ;[1 1 1] Initialisation
  (bind _returnvalue (`GameplayStatics.GetActorOfClass` "/Game/ThirdPerson/Blueprints/BP_ThirdPersonCharacter.BP_ThirdPersonCharacter_C"))
  (set `self.Chara` _returnvalue)
  (bind _returnvalue_2 (`GameplayStatics.GetActorOfClass` "/Game/Blueprints/BP_FinalDoor.BP_FinalDoor_C"))
  (set `self.Door` _returnvalue_2))

(event `self.ReceiveTick`
  (params (DeltaSeconds :type "Float (single-precision)"))
  (if (`self.PlayerIsNear`)
    (if (`self.PlayerCanInteract`)
      (message `/Game/Blueprints/BPI/BPI_Win.OpenDoor` (`self.Door`)))))

(event `self.Collision.OnComponentBeginOverlap`
  (params (OverlappedComponent :type "PrimitiveComponent Object Reference") (OtherActor :type "Actor Object Reference") (OtherComp :type "PrimitiveComponent Object Reference") (OtherBodyIndex :type Integer) (bFromSweep :type Boolean) (SweepResult :type "HitResult Structure (by ref)"))
  ;[1 1 1] Player is here ?
  (if (`self.ActorHasTag` OtherActor "Player")
    (set `self.PlayerIsNear` true)
    (`KismetSystemLibrary.PrintString` "Hello" true true (struct :`R` 0.322618 :`G` 1.0 :`A` 1.0))
    (castclass `/Game/ThirdPerson/Blueprints/BP_ThirdPersonCharacter` "/Game/ThirdPerson/Blueprints/BP_ThirdPersonCharacter.BP_ThirdPersonCharacter_C")))

(event `self.Collision.OnComponentEndOverlap`
  (params (OverlappedComponent :type "PrimitiveComponent Object Reference") (OtherActor :type "Actor Object Reference") (OtherComp :type "PrimitiveComponent Object Reference") (OtherBodyIndex :type Integer))
  ;[1 1 1] Player is here ?
  (if (`self.ActorHasTag` OtherActor "Player")
    (set `self.PlayerIsNear` false)
    (castclass `/Game/ThirdPerson/Blueprints/BP_ThirdPersonCharacter` "/Game/ThirdPerson/Blueprints/BP_ThirdPersonCharacter.BP_ThirdPersonCharacter_C")))

(fn `UserConstructionScript`)